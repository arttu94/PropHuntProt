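; Main menu game mode that shows the WBP_MainMenu widget on BeginPlay with a visible cursor and Game-and-UI input focused on the menu.
; It then prints the path to MyMap.pak under the project's Content/Paks folder, mounts that pak at runtime and calls GetAllMapNames.
; The map name result goes unused, as the loop that prints array entries is disconnected and never runs.
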(event EventBeginPlay
  (bind _returnvalue (Class|KismetSystemLibrary|GetProjectContentDirectory))
  (bind _returnvalue_2 (Game|GetPlayerController 0))
  (bind _returnvalue_3 (Utilities|String|Append _returnvalue "Paks/MyMap.pak"))
  (bind _returnvalue_4 (UserInterface|CreateWidget "/Game/Blueprints/UMG/Menu/WBP_MainMenu.WBP_MainMenu_C"))
  (UserInterface|Viewport|AddtoViewport _returnvalue_4 0)
  (Variables|/Script/Engine.PlayerController|SetbShowMouseCursor _returnvalue_2 true)
  (Input|SetInputModeGameandUI _returnvalue_2 _returnvalue_4 "DoNotLock" false)
  (Development|PrintString _returnvalue_3 true true "(R=0.000000,G=0.660000,B=1.000000,A=1.000000)" 2e+01)
  (Class|GHMainMenuGameMode|MountPak _returnvalue_3)
  (Class|GHMainMenuGameMode|GetAllMapNames))

(event EventTick
  (params (DeltaSeconds :type Float%20%28single-precision%29)))

(fn ConstructionScript)