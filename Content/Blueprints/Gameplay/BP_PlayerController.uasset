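; Player controller for a Prop Hunt game that sets up the local player's HUD, in-game menu and voice chat input.
; On BeginPlay it creates kill feed, match info, crosshair and hidden menu widgets through helpers, one storing references by ref.
; T is push-to-talk, while K or Escape toggles the menu, input mode and cursor.
; A ghost-count updater reads the game state but is unwired in the event graph; KillEvent is empty.
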(event Custom|KillEvent)

(event EventBeginPlay
  (bind _igmenuwidget (Variables|Default|GetIGMenuWidget))
  (if (Pawn|IsLocalController self)
    (CallFunction|CreateAddSetWidget "/Game/Blueprints/UMG/WBP_KillFeed.WBP_KillFeed_C" (Variables|Default|GetKillFeedWidget))
    (CallFunction|CreateAddSetWidget "/Game/Blueprints/UMG/WBP_MatchInfo.WBP_MatchInfo_C" (Variables|Default|GetMatchInfoWidget))
    (CallFunction|CreateAddWidget "/Game/Blueprints/UMG/PlayerCharacter/WBP_Crosshair.WBP_Crosshair_C")
    (CallFunction|CreateAddSetWidget "/Game/Blueprints/UMG/InGameMenu/WBP_IGMenu.WBP_IGMenu_C" _igmenuwidget)
    (Widget|SetVisibility _igmenuwidget "Hidden")
    (Input|SetInputModeGameOnly self)))

(event Input|KeyboardEvents|Escape
  (params (Key :type Key%20Structure))
  (bind _self self)
  (bind _igmenuwidget (Variables|Default|GetIGMenuWidget))
  (:Pressed
    (if (Widget|IsVisible _igmenuwidget)
      (Widget|SetVisibility _igmenuwidget "Hidden")
      (Input|SetInputModeGameOnly _self)
      (Variables|Default|SetbShowMouseCursor false)
      (else
        (Widget|SetVisibility _igmenuwidget "Visible")
        (Input|SetInputModeGameandUI _self _igmenuwidget "DoNotLock" true)
        (Variables|Default|SetbShowMouseCursor true)))))

(event Input|KeyboardEvents|K
  (params (Key :type Key%20Structure))
  (bind _self self)
  (bind _igmenuwidget (Variables|Default|GetIGMenuWidget))
  (:Pressed
    (if (Widget|IsVisible _igmenuwidget)
      (Widget|SetVisibility _igmenuwidget "Hidden")
      (Input|SetInputModeGameOnly _self)
      (Variables|Default|SetbShowMouseCursor false)
      (else
        (Widget|SetVisibility _igmenuwidget "Visible")
        (Input|SetInputModeGameandUI _self _igmenuwidget "DoNotLock" true)
        (Variables|Default|SetbShowMouseCursor true)))))

(event Input|KeyboardEvents|T
  (params (Key :type Key%20Structure))
  (:Pressed
    (Class|AdvancedVoiceLibrary|StartNetworkedVoice))
  (:Released
    (Class|AdvancedVoiceLibrary|StopNetworkedVoice)))

(fn ConstructionScript)

(fn EnableMovement
  (Input|SetIgnoreMoveInput false))

(fn OnRepMatchInfoWidget)

(fn UpdateGhostWidget
  (bind _asbp_prop_hunt_game_state (Utilities|Casting|CastToBP_PropHuntGameState (Game|GetGameState)))
  (Default|UpdateRemainingGhost _asbp_prop_hunt_game_state)
  (Rendering|Components|TextRender|SetText (Variables|/Game/Blueprints/UMG/WBP_MatchInfo.WBP_MatchInfo_C|GetGhostCount (Variables|Default|GetMatchInfoWidget)) (Utilities|Text|ToText(Integer) (Variables|/Game/Blueprints/Gameplay/BP_PropHuntGameState.BP_PropHuntGameState_C|GetRemainingGhost _asbp_prop_hunt_game_state))))

(fn CreateAddWidget
  (params (Class :type User%20Widget%20Class%20Reference))
  (bind _returnvalue (UserInterface|CreateWidget Class self))
  (UserInterface|Viewport|AddtoViewport _returnvalue 0))

(fn CreateAddSetWidget
  (params (Class :type User%20Widget%20Class%20Reference) (WidgetTarget :type User%20Widget%20Object%20Reference%20%28by%20ref%29))
  (bind _returnvalue (UserInterface|CreateWidget Class self))
  (UserInterface|Viewport|AddtoViewport _returnvalue 0)
  (|SetBy-RefVar WidgetTarget _returnvalue))