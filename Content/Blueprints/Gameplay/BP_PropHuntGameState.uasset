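; Game state for a prop hunt match that tracks round time, remaining ghosts and winner announcements.
; Tick copies remaining round time from the game mode, while the ghost count is fetched from it at round start.
; Round start and end use multicasts to hide or show the winner message in the local player controller's match widget.
; A disconnected chain would replace "Prop"-tagged static mesh actors with spawned props, but never runs.
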(event Custom|RoundStart
  (CallFunction|UpdateRemainingGhost)
  (CallFunction|MulticastHideWinnerText))

(event Custom|RoundEnd
  (params (WinnerText :type Name))
  (CallFunction|MulticastDisplayMatchWinners WinnerText))

(event Custom|Multicast_DisplayMatchWinners
  (params (WinnerText :type Name))
  (bind _returnvalue (Game|GetPlayerController 0))
  (if (Pawn|IsLocalPlayerController _returnvalue)
    (bind _asbp_player_controller (Utilities|Casting|CastToBP_PlayerController _returnvalue))
    (Widget|SetVisibility (Variables|/Game/Blueprints/UMG/WBP_MatchInfo.WBP_MatchInfo_C|GetMatchMessage (Variables|/Game/Blueprints/Gameplay/BP_PlayerController.BP_PlayerController_C|GetMatchInfoWidget _asbp_player_controller)) "Visible")
    (Rendering|Components|TextRender|SetText (Variables|/Game/Blueprints/UMG/WBP_MatchInfo.WBP_MatchInfo_C|GetMatchMessage (Variables|/Game/Blueprints/Gameplay/BP_PlayerController.BP_PlayerController_C|GetMatchInfoWidget _asbp_player_controller)) (Utilities|Text|ToText(String) (Utilities|String|Append (Utilities|String|ToString(Text) (Utilities|Text|ToText(Name) WinnerText)) " Win")))))

(event Custom|Multicast_HideWinnerText
  (bind _returnvalue (Game|GetPlayerController 0))
  (if (Pawn|IsLocalPlayerController _returnvalue)
    (bind _asbp_player_controller (Utilities|Casting|CastToBP_PlayerController _returnvalue))
    (Widget|SetVisibility (Variables|/Game/Blueprints/UMG/WBP_MatchInfo.WBP_MatchInfo_C|GetMatchMessage (Variables|/Game/Blueprints/Gameplay/BP_PlayerController.BP_PlayerController_C|GetMatchInfoWidget _asbp_player_controller)) "Hidden")))

(event EventBeginPlay)

(event EventTick
  (params (DeltaSeconds :type Float%20%28single-precision%29))
  (bind _asbp_prop_hunt (Utilities|Casting|CastToBP_PropHunt (Variables|Default|GetAuthorityGameMode)))
  (Variables|Default|SetRemainingTime (Class|GHPropHuntGameMode|GetRemainingRoundTime _asbp_prop_hunt)))

(fn ConstructionScript)

(fn UpdateRemainingGhost
  (bind _authoritygamemode (Variables|Default|GetAuthorityGameMode))
  (if (Utilities|IsValid _authoritygamemode)
    (bind _asghprop_hunt_game_mode (Utilities|Casting|CastToGHPropHuntGameMode _authoritygamemode))
    (bind _returnvalue (Class|GHPropHuntGameMode|GetRemainingGhostPlayerCount _asghprop_hunt_game_mode))
    (Variables|Default|SetRemainingGhost _returnvalue)))

(fn OnRepWinners)