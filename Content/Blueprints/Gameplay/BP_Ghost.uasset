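; BP_Ghost is the Blueprint for a playable ghost, handling its local UI and kill-feed notification in a match.
; After a short delay on BeginPlay, the locally controlled ghost flashes a timed "Hide!" message through the controller's MatchInfoWidget and creates its health bar widget.
; Die triggers the kill feed event on BP_PlayerState, as does the separate CallKillFeedEvent function.
; Destruction removes the health bar from the screen.
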(event EventBeginPlay
  (bind _returnvalue (Pawn|GetController))
  (Utilities|FlowControl|Delay 0.2)
  (if (Utilities|IsValid _returnvalue)
    (if (Pawn|IsLocalController _returnvalue)
      (bind _asbp_player_controller (Utilities|Casting|CastToBP_PlayerController (Pawn|GetController)))
      (Widget|SetVisibility (Variables|/Game/Blueprints/UMG/WBP_MatchInfo.WBP_MatchInfo_C|GetMatchMessage (Variables|/Game/Blueprints/Gameplay/BP_PlayerController.BP_PlayerController_C|GetMatchInfoWidget _asbp_player_controller)) "Visible")
      (Rendering|Components|TextRender|SetText (Variables|/Game/Blueprints/UMG/WBP_MatchInfo.WBP_MatchInfo_C|GetMatchMessage (Variables|/Game/Blueprints/Gameplay/BP_PlayerController.BP_PlayerController_C|GetMatchInfoWidget _asbp_player_controller)) "Hide!")
      (Utilities|Time|SetTimerbyFunctionName 0 "HideMidScreenMessage" 3.0)
      (bind _returnvalue_2 (UserInterface|CreateWidget "/Game/Blueprints/UMG/PlayerCharacter/WBP_GhostHealthBar.WBP_GhostHealthBar_C"))
      (bind _output_get (Variables|Default|SetHealthBarWidget _returnvalue_2))
      (UserInterface|Viewport|AddtoViewport _output_get 0))))

(event EventTick
  (params (DeltaSeconds :type Float%20%28single-precision%29)))

(event EventDie
  (bind _asbp_player_state (Utilities|Casting|CastToBP_PlayerState (Variables|Default|GetPlayerState)))
  (Default|KillFeedEvent _asbp_player_state))

(event EventDestroyed
  (bind _healthbarwidget (Variables|Default|GetHealthBarWidget))
  (if (Utilities|IsValid _healthbarwidget)
    (Widget|RemovefromParent _healthbarwidget)))

(fn ConstructionScript)

(fn CallKillFeedEvent
  (bind _asbp_player_state (Utilities|Casting|CastToBP_PlayerState (Variables|Default|GetPlayerState)))
  (Default|KillFeedEvent _asbp_player_state))

(fn HideMidScreenMessage
  (bind _asbp_player_controller (Utilities|Casting|CastToBP_PlayerController (Pawn|GetController)))
  (Rendering|Components|TextRender|SetText (Variables|/Game/Blueprints/UMG/WBP_MatchInfo.WBP_MatchInfo_C|GetMatchMessage (Variables|/Game/Blueprints/Gameplay/BP_PlayerController.BP_PlayerController_C|GetMatchInfoWidget _asbp_player_controller)) "")
  (Widget|SetVisibility (Variables|/Game/Blueprints/UMG/WBP_MatchInfo.WBP_MatchInfo_C|GetMatchMessage (Variables|/Game/Blueprints/Gameplay/BP_PlayerController.BP_PlayerController_C|GetMatchInfoWidget _asbp_player_controller)) "Hidden"))