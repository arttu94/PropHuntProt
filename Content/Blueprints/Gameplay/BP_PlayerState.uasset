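; BP_PlayerState is a player state Blueprint that reports kills to the kill feed through a single KillFeedEvent.
; The event casts player controller 0 to BP_PlayerController, creates a WBP_KillFeedMessage and adds it to the KillFeedBox of that controller's KillFeedWidget, if valid.
; It then calls KillEvent on the controller.
; The message receives no kill details here.
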(event Custom|KillFeedEvent
  (bind _returnvalue (Game|GetPlayerController 0))
  (if (Utilities|IsValid _returnvalue)
    (bind _asbp_player_controller (Utilities|Casting|CastToBP_PlayerController _returnvalue))
    (Utilities|FlowControl|Sequence
      (:then_0
        (bind _returnvalue_2 (UserInterface|CreateWidget "/Game/Blueprints/UMG/WBP_KillFeedMessage.WBP_KillFeedMessage_C" _asbp_player_controller))
        (if (Utilities|IsValid (Variables|/Game/Blueprints/Gameplay/BP_PlayerController.BP_PlayerController_C|GetKillFeedWidget _asbp_player_controller))
          (Widget|Panel|AddChild (Variables|/Game/Blueprints/UMG/WBP_KillFeed.WBP_KillFeed_C|GetKillFeedBox (Variables|/Game/Blueprints/Gameplay/BP_PlayerController.BP_PlayerController_C|GetKillFeedWidget _asbp_player_controller)) _returnvalue_2)))
      (:then_1
        (Default|KillEvent _asbp_player_controller)))))

(event EventBeginPlay)

(event EventTick
  (params (DeltaSeconds :type Float%20%28single-precision%29)))

(fn ConstructionScript)