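; BP_Hunter is the hunter character in a hunters-versus-ghosts match, handling its local HUD, start-of-round freeze and aim zoom.
; On BeginPlay, after a short delay, the locally controlled hunter gets info and black-screen widgets and ignores move input for FreezeTime.
; A timer then restores movement, removes the black screen and briefly shows a hunt message through the player controller's match widget.
; Right mouse shortens the spring arm for aiming.
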(event EventBeginPlay
  (bind _returnvalue (Pawn|GetController))
  (Utilities|FlowControl|Delay 0.2)
  (if (Utilities|IsValid _returnvalue)
    (if (Pawn|IsLocalController _returnvalue)
      (Utilities|Casting|CastToBP_PlayerController _returnvalue)
      (Utilities|FlowControl|Sequence
        (:then_0
          (CallFunction|CreateWidgets))
        (:then_1
          (Input|SetIgnoreMoveInput (Pawn|GetController) true)
          (Utilities|Time|SetTimerbyFunctionName 0 "RemoveConstrains" (Variables|Movement|GetFreezeTime))
          (bind _output_get (Variables|Default|SetNoADSarml 2e+02))
          (Variables|/Script/Engine.SpringArmComponent|SetTargetArmLength (Variables|Default|GetSpringArmComp) _output_get)
          (Variables|Default|SetADSarml 65.0))))))

(event EventDestroyed
  (bind _hunterinfowidget (Variables|Default|GetHunterInfoWidget))
  (if (Utilities|IsValid _hunterinfowidget)
    (Widget|RemovefromParent _hunterinfowidget)))

(event Input|MouseEvents|RightMouseButton
  (params (Key :type Key%20Structure))
  (bind _springarmcomp (Variables|Default|GetSpringArmComp))
  (:Pressed
    (Variables|/Script/Engine.SpringArmComponent|SetTargetArmLength _springarmcomp (Variables|Default|GetADSarml)))
  (:Released
    (Variables|/Script/Engine.SpringArmComponent|SetTargetArmLength _springarmcomp (Variables|Default|GetNoADSarml))))

(fn ConstructionScript)

(fn RemoveConstrains
  (bind _returnvalue (Pawn|GetController))
  (Input|ResetIgnoreMoveInput _returnvalue)
  (Widget|RemovefromParent (Variables|Default|GetBlackScreen))
  (bind _asbp_player_controller (Utilities|Casting|CastToBP_PlayerController _returnvalue))
  (Widget|SetVisibility (Variables|/Game/Blueprints/UMG/WBP_MatchInfo.WBP_MatchInfo_C|GetMatchMessage (Variables|/Game/Blueprints/Gameplay/BP_PlayerController.BP_PlayerController_C|GetMatchInfoWidget _asbp_player_controller)) "Visible")
  (Rendering|Components|TextRender|SetText (Variables|/Game/Blueprints/UMG/WBP_MatchInfo.WBP_MatchInfo_C|GetMatchMessage (Variables|/Game/Blueprints/Gameplay/BP_PlayerController.BP_PlayerController_C|GetMatchInfoWidget _asbp_player_controller)) "Hunt All Ghosts!")
  (Utilities|Time|SetTimerbyFunctionName 0 "HideMidScreenMessage" 3.0))

(fn HideMidScreenMessage
  (bind _asbp_player_controller (Utilities|Casting|CastToBP_PlayerController (Pawn|GetController)))
  (Rendering|Components|TextRender|SetText (Variables|/Game/Blueprints/UMG/WBP_MatchInfo.WBP_MatchInfo_C|GetMatchMessage (Variables|/Game/Blueprints/Gameplay/BP_PlayerController.BP_PlayerController_C|GetMatchInfoWidget _asbp_player_controller)) "")
  (Widget|SetVisibility (Variables|/Game/Blueprints/UMG/WBP_MatchInfo.WBP_MatchInfo_C|GetMatchMessage (Variables|/Game/Blueprints/Gameplay/BP_PlayerController.BP_PlayerController_C|GetMatchInfoWidget _asbp_player_controller)) "Hidden"))

(fn CreateWidgets
  (bind _returnvalue (UserInterface|CreateWidget "/Game/Blueprints/UMG/PlayerCharacter/WPB_HunterInfo.WPB_HunterInfo_C"))
  (bind _output_get (Variables|Default|SetHunterInfoWidget _returnvalue))
  (UserInterface|Viewport|AddtoViewport _output_get 0)
  (bind _returnvalue_2 (UserInterface|CreateWidget "/Game/Blueprints/UMG/PlayerCharacter/WBP_BlackScreen.WBP_BlackScreen_C"))
  (bind _output_get_2 (Variables|Default|SetBlackScreen _returnvalue_2))
  (UserInterface|Viewport|AddtoViewport _output_get_2 0))