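; BP_PropHunt is the game mode for a Prop Hunt match, tracking players and relaying round events.
; It collects BP_PlayerControllers on post-login and when starting new players, covering seamless travel.
; Round start and end are forwarded to BP_PropHuntGameState, with the match winner passed at round end.
; FreezeHunters and UnFreezeHunters toggle move-input ignore on listed controllers whose pawn is a GHHunter.
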(event EventBeginPlay)

(event EventTick
  (params (DeltaSeconds :type Float%20%28single-precision%29)))

(event EventOnSetMatchState
  (params (NewState :type Name :default "None"))
  (switch name "None"))

(event EventPostLogin
  (params (NewPlayer :type Player%20Controller%20Object%20Reference))
  ;[1 1 1] Add controller on post log in to the controller list
  (bind _asbp_player_controller (Utilities|Casting|CastToBP_PlayerController NewPlayer))
  (Utilities|Array|Add (Variables|Default|GetPlayerControllerList) _asbp_player_controller))

(event EventRoundStart
  (bind _asbp_prop_hunt_game_state (Utilities|Casting|CastToBP_PropHuntGameState (Game|GetGameState)))
  (Default|RoundStart _asbp_prop_hunt_game_state))

(event EventRoundEnd
  (bind _asbp_prop_hunt_game_state (Utilities|Casting|CastToBP_PropHuntGameState (Game|GetGameState)))
  (Default|RoundEnd _asbp_prop_hunt_game_state (Variables|Default|GetMatchWinner)))

(event EventHandleStartingNewPlayer
  (params (NewPlayer :type Player%20Controller%20Object%20Reference))
  ;[1 1 1] Add the controller to the list after the seamless travel
  (bind _asbp_player_controller (Utilities|Casting|CastToBP_PlayerController NewPlayer))
  (Utilities|Array|Add (Variables|Default|GetPlayerControllerList) _asbp_player_controller))

(fn ConstructionScript)

(fn FreezeHunters
  (bind _playercontrollerlist (Variables|Default|GetPlayerControllerList))
  (Development|PrintString (Utilities|String|ToString(Integer) (Utilities|Array|Length _playercontrollerlist)))
  (for _array_element _playercontrollerlist
    (if (Utilities|ClassIsChildOf (Utilities|GetClass (Pawn|GetControlledPawn _array_element)) "/Script/GhostHunt.GHHunter")
      (Input|SetIgnoreMoveInput _array_element true))))

(fn UnFreezeHunters
  (for _array_element (Variables|Default|GetPlayerControllerList)
    (if (Utilities|ClassIsChildOf (Utilities|GetClass (Pawn|GetControlledPawn _array_element)) "/Script/GhostHunt.GHHunter")
      (Input|SetIgnoreMoveInput _array_element false))))