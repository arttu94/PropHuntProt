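; Player controller, named for the main menu, that provides an in-game menu widget toggled with Escape.
; On BeginPlay it sets UI-only input without locking the mouse, then creates WBP_IGMenu, stores it and adds it to the viewport hidden.
; An Escape press flips the widget between visible and hidden, with no change to input mode.
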(event EventBeginPlay
  (Input|SetInputModeUIOnly self 0 "DoNotLock")
  (bind _returnvalue (UserInterface|CreateWidget "/Game/Blueprints/UMG/InGameMenu/WBP_IGMenu.WBP_IGMenu_C"))
  (bind _output_get (Variables|Default|SetIGMenuWidget _returnvalue))
  (Widget|SetVisibility _output_get "Hidden")
  (UserInterface|Viewport|AddtoViewport _output_get 0))

(event EventTick
  (params (DeltaSeconds :type Float%20%28single-precision%29)))

(event Input|KeyboardEvents|Escape
  (params (Key :type Key%20Structure))
  (bind _igmenuwidget (Variables|Default|GetIGMenuWidget))
  (:Pressed
    (if (Widget|IsVisible _igmenuwidget)
      (Widget|SetVisibility _igmenuwidget "Hidden")
      (else
        (Widget|SetVisibility _igmenuwidget "Visible")))))

(fn ConstructionScript)